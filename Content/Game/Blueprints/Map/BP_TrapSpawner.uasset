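; BP_TrapSpawner is a map Blueprint that spawns a trap and randomizes its spike timing when play begins.
; On BeginPlay it calls SpawnActor and casts the result to SpikeTrap.
; It sets random show, close, reset and re-show delays on the trap before calling FinishSpawning, so each spawned trap gets its own rhythm.
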(event `self.ReceiveBeginPlay`
  (bind _returnvalue (`self.SpawnActor`))
  (bind _asspike_trap (cast `SpikeTrap` _returnvalue))
  (`/Engine/EditorBlueprintResources/StandardMacros.IsValid` _asspike_trap
    (:`Is Valid`
      (`SpikeTrap.SetTimeToShow` _asspike_trap (`KismetMathLibrary.RandomFloatInRange` 0.2 0.5))
      (`SpikeTrap.SetTimeToClose` _asspike_trap (`KismetMathLibrary.RandomFloatInRange` 0.5 2.0))
      (`SpikeTrap.SetTimeToResetSpikesAfterShowing` _asspike_trap (`KismetMathLibrary.RandomFloatInRange` 2.5 5.0))
      (`SpikeTrap.SetTimeToShowSpikesAfterClosing` _asspike_trap (`KismetMathLibrary.RandomFloatInRange` 0.5 1.0))
      (`self.FinishSpawning` _asspike_trap))))

(fn `UserConstructionScript`)